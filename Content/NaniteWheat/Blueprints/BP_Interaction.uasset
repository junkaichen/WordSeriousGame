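; Template actor logic, marked for copying, that feeds player movement into MPC_NaniteFoliageController for interactive Nanite wheat foliage.
; Each Tick eases a moving value toward 1 or 0 by a velocity threshold, using a randomized interpolation speed to vary bounce-back.
; It writes that value raw to "Interaction Status" and clamped to "IsMoving", whose minimum limits recovery, and sends the actor location as "PlayerPosition".
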(event `self.ReceiveTick`
  (params (DeltaSeconds :type "Float (single-precision)"))
  ;[1 1 1 1 98] Copy this
  (`|ExecutionSequence`
    (:`then_0`
      (bind _output_get (set `self.TransitionSpeed` (`KismetMathLibrary.RandomFloatInRange` 1.0 8.0)))
      (if (> (`KismetMathLibrary.VSize` (`self.GetVelocity`)) 200.0)
        (set `self.IsMoving` 1.0)
        (else
          (set `self.IsMoving` 0.0)))
      (bind _output_get_2 (set `self.CurrentSpeed` (`KismetMathLibrary.FInterpTo` (`self.CurrentSpeed`) (`self.IsMoving`) DeltaSeconds _output_get)))
      (`KismetMaterialLibrary.SetScalarParameterValue` "/Game/NaniteWheat/Materials/MaterialParameterCollection/MPC_NaniteFoliageController.MPC_NaniteFoliageController" "IsMoving" (`KismetMathLibrary.FClamp` _output_get_2 0.25))
      (`KismetMaterialLibrary.SetScalarParameterValue` "/Game/NaniteWheat/Materials/MaterialParameterCollection/MPC_NaniteFoliageController.MPC_NaniteFoliageController" "Interaction Status" _output_get_2))
    (:`then_1`
      ;;[1 1 1] Set current player location
      (`KismetMaterialLibrary.SetVectorParameterValue` "/Game/NaniteWheat/Materials/MaterialParameterCollection/MPC_NaniteFoliageController.MPC_NaniteFoliageController" "PlayerPosition" (`KismetMathLibrary.Conv_VectorToLinearColor` (`self.K2_GetActorLocation`))))))

(fn `UserConstructionScript`)