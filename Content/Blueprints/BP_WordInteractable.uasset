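; BP_WordInteractable is an interactable actor that carries word data and can be collected once.
; CanBeInteracted returns true only while CanInteract is set and the word has not been collected, and GetWordData exposes the stored WordData.
; OnCollected sets IsCollected and disables collision on its Sphere component.
; The event graph and construction script are empty, so other code must call these functions.
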(fn `CanBeInteracted`
  (returns (CanBeInteracted :type Boolean))
  (return (and (`self.CanInteract`) (not (`self.IsCollected`)))))

(fn `GetWordData`
  (returns (NewParam :type "/Game/Blueprints/Struct_WordData Structure"))
  (return (`self.WordData`)))

(fn `OnCollected`
  (set `self.IsCollected` true)
  (`PrimitiveComponent.SetCollisionEnabled` (`self.Sphere`) "NoCollision"))

(fn `UserConstructionScript`)