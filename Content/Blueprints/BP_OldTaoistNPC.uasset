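; BP_OldTaoistNPC is an NPC, named as an old Taoist, that the first-person player can talk to when nearby.
; A Box overlap flags the player as in range and sets or clears itself as the character's CurrentTalkNPC.
; StartDialogue, guarded by range and talking flags, creates a WBP_Dialogue widget and passes it the dialogue lines.
; OnDialogueFinished removes the widget, resets the talking state and notifies the player character.
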(event `self.Box.OnComponentBeginOverlap`
  (params (OverlappedComponent :type "PrimitiveComponent Object Reference") (OtherActor :type "Actor Object Reference") (OtherComp :type "PrimitiveComponent Object Reference") (OtherBodyIndex :type Integer) (bFromSweep :type Boolean) (SweepResult :type "HitResult Structure (by ref)"))
  (bind _asbp_first_person_character (cast `/Game/FirstPerson/Blueprints/BP_FirstPersonCharacter` OtherActor))
  (set `self.bPlayerInRange` true)
  (set `/Game/FirstPerson/Blueprints/BP_FirstPersonCharacter.CurrentTalkNPC` self _asbp_first_person_character))

(event `self.Box.OnComponentEndOverlap`
  (params (OverlappedComponent :type "PrimitiveComponent Object Reference") (OtherActor :type "Actor Object Reference") (OtherComp :type "PrimitiveComponent Object Reference") (OtherBodyIndex :type Integer))
  (bind _asbp_first_person_character (cast `/Game/FirstPerson/Blueprints/BP_FirstPersonCharacter` OtherActor))
  (set `self.bPlayerInRange` false)
  (set `/Game/FirstPerson/Blueprints/BP_FirstPersonCharacter.CurrentTalkNPC` null _asbp_first_person_character))

(event `StartDialogue`
  (if (`self.bPlayerInRange`)
    (if (not (`self.bIsTalking`))
      (set `self.bIsTalking` true)
      (bind _returnvalue (`|CreateWidget` "/Game/Blueprints/WBP_Dialogue.WBP_Dialogue_C"))
      (bind _output_get (set `self.CurrentDialogueWideget` _returnvalue))
      (`UserWidget.AddToViewport` _output_get 0)
      (`/Game/Blueprints/WBP_Dialogue.SetDialogueData` (`self.CurrentDialogueWideget`) (`self.DialogueLoines`)))))

(event `OnDialogueFinished`
  (set `self.bIsTalking` false)
  (`Widget.RemoveFromParent` (`self.CurrentDialogueWideget`))
  (set `self.CurrentDialogueWideget` null)
  (bind _asbp_first_person_character (cast `/Game/FirstPerson/Blueprints/BP_FirstPersonCharacter` (`GameplayStatics.GetPlayerCharacter` 0)))
  (`/Game/FirstPerson/Blueprints/BP_FirstPersonCharacter.DialogueFinished` _asbp_first_person_character))

(fn `UserConstructionScript`)